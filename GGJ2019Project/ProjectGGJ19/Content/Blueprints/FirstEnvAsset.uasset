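; Environment rock actor that fades in and out through the Width scalar parameter on Rock1's material.
; BeginPlay sets Width to 1, then Tick steps FadeValue by per-frame speeds according to FadeState, which is not triggered in this file.
; Both limits set collision to QueryAndPhysics and stop the fade.
; Tick calls CreateDynamicMaterialInstance on each fade update rather than caching the instance.
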(event EventTick
  (params (DeltaSeconds :type Float%20%28single-precision%29))
  (switch Utilities|FlowControl|Switch|SwitchonFadeState (Variables|Default|GetFadeState)
    (:NewEnumerator0
      ;[1 1 1] FadeOut
      (if (< (Variables|Default|GetFadeValue) 1.0)
        (Variables|Default|SetFadeValue (+ (Variables|Default|GetFadeValue) (Variables|Default|GetFadeOutSpeed)))
        (else
          (Variables|Default|SetFadeValue 1.0)
          (Collision|SetCollisionEnabled (Variables|Default|GetRock1) "QueryAndPhysics")
          (Variables|Default|SetFadeState "NewEnumerator2" :!label _label))))
    (:NewEnumerator1
      ;[1 1 1] FadeIn
      (if (> (Variables|Default|GetFadeValue) 0.0)
        (Variables|Default|SetFadeValue (- (Variables|Default|GetFadeValue) (Variables|Default|GetFadeInSpeed)))
        (else
          (Variables|Default|SetFadeValue 0.0)
          (Collision|SetCollisionEnabled (Variables|Default|GetRock1) "QueryAndPhysics")
          (goto _label)))))
  ;[1 1 1] Change material
  (bind _returnvalue (Rendering|Material|CreateDynamicMaterialInstance (Variables|Default|GetRock1) 0 0 "None" :!class /Script/Engine.PrimitiveComponent))
  (Rendering|Material|SetScalarParameterValue _returnvalue "Width" (Variables|Default|GetFadeValue) :!class /Script/Engine.MaterialInstanceDynamic))

(event EventBeginPlay
  (bind _returnvalue (Rendering|Material|CreateDynamicMaterialInstance (Variables|Default|GetRock1) 0 0 "None" :!class /Script/Engine.PrimitiveComponent))
  (Rendering|Material|SetScalarParameterValue _returnvalue "Width" 1.0 :!class /Script/Engine.MaterialInstanceDynamic))

(event Collision|EventActorBeginOverlap
  (params (OtherActor :type Actor%20Object%20Reference)))

(fn ConstructionScript)