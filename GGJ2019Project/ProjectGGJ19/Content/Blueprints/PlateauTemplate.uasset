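; Plateau template actor that fades a platform mesh in and out with a cracked-edge dissolve effect.
; FadeOut creates a dynamic material, then chains timelines driving crack "Amount" and dissolve "Width" before disabling collision.
; FadeIn runs the reverse sequence and re-enables collision at the end.
; After FadeOut, a marked hack clears the ThirdPersonCharacter's Switching flag and prints a debug message.
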(event Custom|FadeOut
  (bind _returnvalue (Rendering|Material|CreateDynamicMaterialInstance (Variables|Default|GetPlateauMesh) 0 0 "None" :!class /Script/Engine.PrimitiveComponent))
  ;[1 1 1] Cracked line/edge appearance time
  (bind _edgeshowvalue (Timeline|Timeline_ShowCracks PlayFromStart)
    (:Update
      (Rendering|Material|SetScalarParameterValue _returnvalue "Amount" _edgeshowvalue :!class /Script/Engine.MaterialInstanceDynamic))
    (:Finished
      ;[1 1 1] Texture dissolve
      (bind _dissolvevalue (Timeline|Timeline_dissolveTexture PlayFromStart)
        (:Update
          (Rendering|Material|SetScalarParameterValue _returnvalue "Width" _dissolvevalue :!class /Script/Engine.MaterialInstanceDynamic))
        (:Finished
          (Collision|SetCollisionEnabled (Variables|Default|GetPlateauMesh) "NoCollision")
          ;[1 1 1] Hack
          (bind _asthird_person_character (Utilities|Casting|CastToThirdPersonCharacter (Game|GetPlayerCharacter 0)))
          (Variables|/Game/ThirdPersonBP/Blueprints/ThirdPersonCharacter.ThirdPersonCharacter_C|SetSwitching _asthird_person_character false)
          (Development|PrintString "Switch False!"))))))

(event Custom|FadeIn
  (bind _returnvalue (Rendering|Material|CreateDynamicMaterialInstance (Variables|Default|GetPlateauMesh) 0 0 "None" :!class /Script/Engine.PrimitiveComponent))
  ;[1 1 1] Texture resolve
  (bind _resolvevalue (Timeline|Timeline_resolveTexture PlayFromStart)
    (:Update
      (Rendering|Material|SetScalarParameterValue _returnvalue "Width" _resolvevalue :!class /Script/Engine.MaterialInstanceDynamic))
    (:Finished
      ;[1 1 1] Cracked line/edge disappearance time
      (bind _edgehidevalue (Timeline|Timeline_HideCracks PlayFromStart)
        (:Update
          (Rendering|Material|SetScalarParameterValue _returnvalue "Amount" _edgehidevalue :!class /Script/Engine.MaterialInstanceDynamic))
        (:Finished
          (Collision|SetCollisionEnabled (Variables|Default|GetPlateauMesh) "QueryAndPhysics"))))))

(fn ConstructionScript)